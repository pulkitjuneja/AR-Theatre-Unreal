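; Networked particle actor that drives number particle effects from incoming OSC messages, apparently as an audio-frequency visualizer.
; On BeginPlay, only the server instance opens an OSC server on the machine IP.
; "P" addresses pass a float to SpawnNumbers, which sets banded spawn rates and calls VelocityNumbers and AccelerationNumbers for randomized, intensity-scaled motion across several emitters.
; "S" addresses trigger a ServerTravel to the Quartet map.
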(event `self.ReceiveBeginPlay`
  (bind _asbp_game_instace (cast `/Game/Blueprints/BP_GameInstace` (`GameplayStatics.GetGameInstance`)))
  (if (`/Game/Blueprints/BP_GameInstace.isServer` _asbp_game_instace)
    (`KismetSystemLibrary.PrintString` "Creating osc server")
    (bind _returnvalue (`OSCManager.CreateOSCServer` (`/Game/Blueprints/BP_GameInstace.MachineIP` _asbp_game_instace) 7000 false true "" null))
    (`KismetSystemLibrary.PrintString` "OSC server created")
    (bind _output_get (set `self.OscServer` _returnvalue))
    (clear `OSCServer.OnOscBundleReceived` _output_get)
    (add `OSCServer.OnOscMessageReceived` _output_get (`|CreateDelegate` :!event `OSCMessageReceived`))))

(event `OSCMessageReceived`
  (params (Message :type "OSCMessage Structure (by ref)") (IPAddress :type String) (Port :type Integer))
  (bind _returnvalue (`OSCManager.GetOSCMessageAddress` Message))
  (bind _returnvalue_2 (`OSCManager.GetOSCAddressFullPath` _returnvalue))
  (`|ExecutionSequence`
    (:`then_0`
      (bind _returnvalue_3 (`KismetStringLibrary.GetSubstring` _returnvalue_2 1))
      (if (`KismetStringLibrary.EqualEqual_StrStr` _returnvalue_3 "P")
        (bind _value (`OSCManager.GetFloat` Message))
        (`self.Spawn Effects` _value)))
    (:`then_1`
      (if (`KismetStringLibrary.EqualEqual_StrStr` _returnvalue_3 "S")
        (`KismetSystemLibrary.PrintString` "Switching")
        (`KismetSystemLibrary.ExecuteConsoleCommand` "ServerTravel Quartet" null)))))

(event `Spawn Effects`
  (params (Frequency :type "Float (double-precision)"))
  (`self.Spawn Numbers` (* Frequency 1.0)))

(fn `Acceleration Numbers`
  (params (freq_notes_acc :type "Float (double-precision)"))
  (bind _returnvalue (`KismetMathLibrary.MakeVector` (`KismetMathLibrary.RandomFloatInRange` -2.0 2.0) 0.0 freq_notes_acc))
  (bind _returnvalue_2 (`KismetMathLibrary.MakeVector` (`KismetMathLibrary.RandomFloatInRange` -10.0 10.0) 5.0 (`KismetMathLibrary.RandomFloatInRange` 0.0 15.0)))
  (bind _returnvalue_3 (`KismetMathLibrary.MakeVector` (`KismetMathLibrary.RandomFloatInRange` -6.0 6.0) 0.0 freq_notes_acc))
  (if (<= freq_notes_acc 10.0)
    (`FXSystemComponent.SetVectorParameter` (`self.Number_Particles`) "0_acc" _returnvalue)
    (`FXSystemComponent.SetVectorParameter` (`self.Number_Particles1`) "0_acc" _returnvalue)
    (`FXSystemComponent.SetVectorParameter` (`self.Number_Particles4`) "0_acc" _returnvalue)
    (`FXSystemComponent.SetVectorParameter` (`self.Number_Particles3`) "0_acc" _returnvalue)
    (`FXSystemComponent.SetVectorParameter` (`self.Number_Particles2`) "0_acc" _returnvalue)
    (`FXSystemComponent.SetVectorParameter` (`self.Number_Particles`) "1_acc" _returnvalue)
    (`FXSystemComponent.SetVectorParameter` (`self.Number_Particles1`) "1_acc" _returnvalue)
    (`FXSystemComponent.SetVectorParameter` (`self.Number_Particles4`) "1_acc" _returnvalue)
    (`FXSystemComponent.SetVectorParameter` (`self.Number_Particles3`) "1_acc" _returnvalue)
    (`FXSystemComponent.SetVectorParameter` (`self.Number_Particles2`) "1_acc" _returnvalue)
    (`FXSystemComponent.SetVectorParameter` (`self.Number_Particles`) "2_acc" _returnvalue)
    (`FXSystemComponent.SetVectorParameter` (`self.Number_Particles1`) "2_acc" _returnvalue)
    (`FXSystemComponent.SetVectorParameter` (`self.Number_Particles4`) "2_acc" _returnvalue)
    (`FXSystemComponent.SetVectorParameter` (`self.Number_Particles3`) "2_acc" _returnvalue)
    (`FXSystemComponent.SetVectorParameter` (`self.Number_Particles2`) "2_acc" _returnvalue)
    (`FXSystemComponent.SetVectorParameter` (`self.Number_Particles`) "3_acc" _returnvalue)
    (`FXSystemComponent.SetVectorParameter` (`self.Number_Particles1`) "3_acc" _returnvalue)
    (`FXSystemComponent.SetVectorParameter` (`self.Number_Particles4`) "3_acc" _returnvalue)
    (`FXSystemComponent.SetVectorParameter` (`self.Number_Particles3`) "3_acc" _returnvalue)
    (`FXSystemComponent.SetVectorParameter` (`self.Number_Particles2`) "3_acc" _returnvalue)
    (`FXSystemComponent.SetVectorParameter` (`self.Number_Particles`) "4_acc" _returnvalue)
    (`FXSystemComponent.SetVectorParameter` (`self.Number_Particles1`) "4_acc" _returnvalue)
    (`FXSystemComponent.SetVectorParameter` (`self.Number_Particles4`) "4_acc" _returnvalue)
    (`FXSystemComponent.SetVectorParameter` (`self.Number_Particles3`) "4_acc" _returnvalue)
    (`FXSystemComponent.SetVectorParameter` (`self.Number_Particles2`) "4_acc" _returnvalue)
    (`FXSystemComponent.SetVectorParameter` (`self.Number_Particles`) "5_acc" _returnvalue)
    (`FXSystemComponent.SetVectorParameter` (`self.Number_Particles1`) "5_acc" _returnvalue)
    (`FXSystemComponent.SetVectorParameter` (`self.Number_Particles4`) "5_acc" _returnvalue)
    (`FXSystemComponent.SetVectorParameter` (`self.Number_Particles3`) "5_acc" _returnvalue)
    (`FXSystemComponent.SetVectorParameter` (`self.Number_Particles2`) "5_acc" _returnvalue)
    (elif (<= freq_notes_acc 20.0)
      (`FXSystemComponent.SetVectorParameter` (`self.Number_Particles`) "0_acc" _returnvalue_3)
      (`FXSystemComponent.SetVectorParameter` (`self.Number_Particles1`) "0_acc" _returnvalue_3)
      (`FXSystemComponent.SetVectorParameter` (`self.Number_Particles4`) "0_acc" _returnvalue_3)
      (`FXSystemComponent.SetVectorParameter` (`self.Number_Particles3`) "0_acc" _returnvalue_3)
      (`FXSystemComponent.SetVectorParameter` (`self.Number_Particles2`) "0_acc" _returnvalue_3)
      (`FXSystemComponent.SetVectorParameter` (`self.Number_Particles`) "1_acc" _returnvalue_3)
      (`FXSystemComponent.SetVectorParameter` (`self.Number_Particles1`) "1_acc" _returnvalue_3)
      (`FXSystemComponent.SetVectorParameter` (`self.Number_Particles4`) "1_acc" _returnvalue_3)
      (`FXSystemComponent.SetVectorParameter` (`self.Number_Particles3`) "1_acc" _returnvalue_3)
      (`FXSystemComponent.SetVectorParameter` (`self.Number_Particles2`) "1_acc" _returnvalue_3)
      (`FXSystemComponent.SetVectorParameter` (`self.Number_Particles`) "2_acc" _returnvalue_3)
      (`FXSystemComponent.SetVectorParameter` (`self.Number_Particles1`) "2_acc" _returnvalue_3)
      (`FXSystemComponent.SetVectorParameter` (`self.Number_Particles4`) "2_acc" _returnvalue_3)
      (`FXSystemComponent.SetVectorParameter` (`self.Number_Particles3`) "2_acc" _returnvalue_3)
      (`FXSystemComponent.SetVectorParameter` (`self.Number_Particles2`) "2_acc" _returnvalue_3)
      (`FXSystemComponent.SetVectorParameter` (`self.Number_Particles`) "3_acc" _returnvalue_3)
      (`FXSystemComponent.SetVectorParameter` (`self.Number_Particles1`) "3_acc" _returnvalue_3)
      (`FXSystemComponent.SetVectorParameter` (`self.Number_Particles4`) "3_acc" _returnvalue_3)
      (`FXSystemComponent.SetVectorParameter` (`self.Number_Particles3`) "3_acc" _returnvalue_3)
      (`FXSystemComponent.SetVectorParameter` (`self.Number_Particles2`) "3_acc" _returnvalue_3)
      (`FXSystemComponent.SetVectorParameter` (`self.Number_Particles`) "4_acc" _returnvalue_3)
      (`FXSystemComponent.SetVectorParameter` (`self.Number_Particles1`) "4_acc" _returnvalue_3)
      (`FXSystemComponent.SetVectorParameter` (`self.Number_Particles4`) "4_acc" _returnvalue_3)
      (`FXSystemComponent.SetVectorParameter` (`self.Number_Particles3`) "4_acc" _returnvalue_3)
      (`FXSystemComponent.SetVectorParameter` (`self.Number_Particles2`) "4_acc" _returnvalue_3)
      (`FXSystemComponent.SetVectorParameter` (`self.Number_Particles`) "5_acc" _returnvalue_3)
      (`FXSystemComponent.SetVectorParameter` (`self.Number_Particles1`) "5_acc" _returnvalue_3)
      (`FXSystemComponent.SetVectorParameter` (`self.Number_Particles4`) "5_acc" _returnvalue_3)
      (`FXSystemComponent.SetVectorParameter` (`self.Number_Particles3`) "5_acc" _returnvalue_3)
      (`FXSystemComponent.SetVectorParameter` (`self.Number_Particles2`) "5_acc" _returnvalue_3)
      (elif (> freq_notes_acc 20.0)
        (`FXSystemComponent.SetVectorParameter` (`self.Number_Particles`) "0_acc" _returnvalue_2)
        (`FXSystemComponent.SetVectorParameter` (`self.Number_Particles1`) "0_acc" _returnvalue_2)
        (`FXSystemComponent.SetVectorParameter` (`self.Number_Particles4`) "0_acc" _returnvalue_2)
        (`FXSystemComponent.SetVectorParameter` (`self.Number_Particles3`) "0_acc" _returnvalue_2)
        (`FXSystemComponent.SetVectorParameter` (`self.Number_Particles2`) "0_acc" _returnvalue_2)
        (`FXSystemComponent.SetVectorParameter` (`self.Number_Particles`) "1_acc" _returnvalue_2)
        (`FXSystemComponent.SetVectorParameter` (`self.Number_Particles1`) "1_acc" _returnvalue_2)
        (`FXSystemComponent.SetVectorParameter` (`self.Number_Particles4`) "1_acc" _returnvalue_2)
        (`FXSystemComponent.SetVectorParameter` (`self.Number_Particles3`) "1_acc" _returnvalue_2)
        (`FXSystemComponent.SetVectorParameter` (`self.Number_Particles2`) "1_acc" _returnvalue_2)
        (`FXSystemComponent.SetVectorParameter` (`self.Number_Particles`) "2_acc" _returnvalue_2)
        (`FXSystemComponent.SetVectorParameter` (`self.Number_Particles1`) "2_acc" _returnvalue_2)
        (`FXSystemComponent.SetVectorParameter` (`self.Number_Particles4`) "2_acc" _returnvalue_2)
        (`FXSystemComponent.SetVectorParameter` (`self.Number_Particles3`) "2_acc" _returnvalue_2)
        (`FXSystemComponent.SetVectorParameter` (`self.Number_Particles2`) "2_acc" _returnvalue_2)
        (`FXSystemComponent.SetVectorParameter` (`self.Number_Particles`) "3_acc" _returnvalue_2)
        (`FXSystemComponent.SetVectorParameter` (`self.Number_Particles1`) "3_acc" _returnvalue_2)
        (`FXSystemComponent.SetVectorParameter` (`self.Number_Particles4`) "3_acc" _returnvalue_2)
        (`FXSystemComponent.SetVectorParameter` (`self.Number_Particles3`) "3_acc" _returnvalue_2)
        (`FXSystemComponent.SetVectorParameter` (`self.Number_Particles2`) "3_acc" _returnvalue_2)
        (`FXSystemComponent.SetVectorParameter` (`self.Number_Particles`) "4_acc" _returnvalue_2)
        (`FXSystemComponent.SetVectorParameter` (`self.Number_Particles1`) "4_acc" _returnvalue_2)
        (`FXSystemComponent.SetVectorParameter` (`self.Number_Particles4`) "4_acc" _returnvalue_2)
        (`FXSystemComponent.SetVectorParameter` (`self.Number_Particles3`) "4_acc" _returnvalue_2)
        (`FXSystemComponent.SetVectorParameter` (`self.Number_Particles2`) "4_acc" _returnvalue_2)
        (`FXSystemComponent.SetVectorParameter` (`self.Number_Particles`) "5_acc" _returnvalue_2)
        (`FXSystemComponent.SetVectorParameter` (`self.Number_Particles1`) "5_acc" _returnvalue_2)
        (`FXSystemComponent.SetVectorParameter` (`self.Number_Particles4`) "5_acc" _returnvalue_2)
        (`FXSystemComponent.SetVectorParameter` (`self.Number_Particles3`) "5_acc" _returnvalue_2)
        (`FXSystemComponent.SetVectorParameter` (`self.Number_Particles2`) "5_acc" _returnvalue_2)))))

(fn `PrintFrequency`
  (params (frequency :type "Float (double-precision)")))

(fn `Spawn Numbers`
  (params (freq_spawn_notes :type "Float (double-precision)"))
  (bind _returnvalue (* freq_spawn_notes 100.0))
  (bind _returnvalue_2 (`KismetMathLibrary.Round` _returnvalue))
  (bind _returnvalue_3 (* _returnvalue 1.0))
  (if (< _returnvalue_2 1)
    (`FXSystemComponent.SetFloatParameter` (`self.Number_Particles`) "0_spawn" 0.0)
    (`FXSystemComponent.SetFloatParameter` (`self.Number_Particles3`) "0_spawn" 0.0)
    (`FXSystemComponent.SetFloatParameter` (`self.Number_Particles4`) "0_spawn" 0.0)
    (`FXSystemComponent.SetFloatParameter` (`self.Number_Particles1`) "0_spawn" 0.0)
    (`FXSystemComponent.SetFloatParameter` (`self.Number_Particles`) "1_spawn" 0.0)
    (`FXSystemComponent.SetFloatParameter` (`self.Number_Particles1`) "1_spawn" 0.0)
    (`FXSystemComponent.SetFloatParameter` (`self.Number_Particles4`) "1_spawn" 0.0)
    (`FXSystemComponent.SetFloatParameter` (`self.Number_Particles3`) "1_spawn" 0.0)
    (`FXSystemComponent.SetFloatParameter` (`self.Number_Particles`) "2_spawn" 0.0)
    (`FXSystemComponent.SetFloatParameter` (`self.Number_Particles1`) "2_spawn" 0.0)
    (`FXSystemComponent.SetFloatParameter` (`self.Number_Particles4`) "2_spawn" 0.0)
    (`FXSystemComponent.SetFloatParameter` (`self.Number_Particles`) "3_spawn" 0.0)
    (`FXSystemComponent.SetFloatParameter` (`self.Number_Particles1`) "3_spawn" 0.0)
    (`FXSystemComponent.SetFloatParameter` (`self.Number_Particles4`) "3_spawn" 0.0)
    (`FXSystemComponent.SetFloatParameter` (`self.Number_Particles`) "4_spawn" 0.0)
    (`FXSystemComponent.SetFloatParameter` (`self.Number_Particles1`) "4_spawn" 0.0)
    (`FXSystemComponent.SetFloatParameter` (`self.Number_Particles4`) "4_spawn" 0.0)
    (`FXSystemComponent.SetFloatParameter` (`self.Number_Particles3`) "4_spawn" 0.0)
    (`FXSystemComponent.SetFloatParameter` (`self.Number_Particles`) "5_spawn" 0.0)
    (`FXSystemComponent.SetFloatParameter` (`self.Number_Particles1`) "5_spawn" 0.0)
    (`FXSystemComponent.SetFloatParameter` (`self.Number_Particles4`) "5_spawn" 0.0)
    (`FXSystemComponent.SetFloatParameter` (`self.Number_Particles3`) "5_spawn" 0.0)
    (`self.Velocity Numbers` 0.0)
    (`self.Acceleration Numbers` 0.0)
    (elif (<= _returnvalue_2 5)
      (`FXSystemComponent.SetFloatParameter` (`self.Number_Particles`) "0_spawn" 0.5)
      (`FXSystemComponent.SetFloatParameter` (`self.Number_Particles1`) "0_spawn" 0.5)
      (`FXSystemComponent.SetFloatParameter` (`self.Number_Particles4`) "0_spawn" 0.5)
      (`FXSystemComponent.SetFloatParameter` (`self.Number_Particles3`) "0_spawn" 0.5)
      (`FXSystemComponent.SetFloatParameter` (`self.Number_Particles`) "1_spawn" 0.5)
      (`FXSystemComponent.SetFloatParameter` (`self.Number_Particles1`) "1_spawn" 0.5)
      (`FXSystemComponent.SetFloatParameter` (`self.Number_Particles4`) "1_spawn" 0.5)
      (`FXSystemComponent.SetFloatParameter` (`self.Number_Particles3`) "1_spawn" 0.5)
      (`FXSystemComponent.SetFloatParameter` (`self.Number_Particles`) "2_spawn" 0.5)
      (`FXSystemComponent.SetFloatParameter` (`self.Number_Particles1`) "2_spawn" 0.5)
      (`FXSystemComponent.SetFloatParameter` (`self.Number_Particles4`) "2_spawn" 0.5)
      (`FXSystemComponent.SetFloatParameter` (`self.Number_Particles`) "3_spawn" 0.5)
      (`FXSystemComponent.SetFloatParameter` (`self.Number_Particles1`) "3_spawn" 0.5)
      (`FXSystemComponent.SetFloatParameter` (`self.Number_Particles4`) "3_spawn" 0.5)
      (`FXSystemComponent.SetFloatParameter` (`self.Number_Particles`) "4_spawn" 0.5)
      (`FXSystemComponent.SetFloatParameter` (`self.Number_Particles1`) "4_spawn" 0.5)
      (`FXSystemComponent.SetFloatParameter` (`self.Number_Particles4`) "4_spawn" 0.5)
      (`FXSystemComponent.SetFloatParameter` (`self.Number_Particles3`) "4_spawn" 0.5)
      (`FXSystemComponent.SetFloatParameter` (`self.Number_Particles`) "5_spawn" 0.5)
      (`FXSystemComponent.SetFloatParameter` (`self.Number_Particles1`) "5_spawn" 0.5)
      (`FXSystemComponent.SetFloatParameter` (`self.Number_Particles4`) "5_spawn" 0.5)
      (`FXSystemComponent.SetFloatParameter` (`self.Number_Particles3`) "5_spawn" 0.5)
      (`self.Velocity Numbers` _returnvalue)
      (`self.Acceleration Numbers` _returnvalue)
      (elif (<= _returnvalue_2 10)
        (`FXSystemComponent.SetFloatParameter` (`self.Number_Particles`) "0_spawn" 2.0)
        (`FXSystemComponent.SetFloatParameter` (`self.Number_Particles1`) "0_spawn" 2.0)
        (`FXSystemComponent.SetFloatParameter` (`self.Number_Particles4`) "0_spawn" 2.0)
        (`FXSystemComponent.SetFloatParameter` (`self.Number_Particles3`) "0_spawn" 2.0)
        (`FXSystemComponent.SetFloatParameter` (`self.Number_Particles`) "1_spawn" 2.0)
        (`FXSystemComponent.SetFloatParameter` (`self.Number_Particles1`) "1_spawn" 2.0)
        (`FXSystemComponent.SetFloatParameter` (`self.Number_Particles4`) "1_spawn" 2.0)
        (`FXSystemComponent.SetFloatParameter` (`self.Number_Particles3`) "1_spawn" 2.0)
        (`FXSystemComponent.SetFloatParameter` (`self.Number_Particles`) "2_spawn" 2.0)
        (`FXSystemComponent.SetFloatParameter` (`self.Number_Particles1`) "2_spawn" 2.0)
        (`FXSystemComponent.SetFloatParameter` (`self.Number_Particles4`) "2_spawn" 2.0)
        (`FXSystemComponent.SetFloatParameter` (`self.Number_Particles`) "3_spawn" 2.0)
        (`FXSystemComponent.SetFloatParameter` (`self.Number_Particles1`) "3_spawn" 2.0)
        (`FXSystemComponent.SetFloatParameter` (`self.Number_Particles4`) "3_spawn" 2.0)
        (`FXSystemComponent.SetFloatParameter` (`self.Number_Particles`) "4_spawn" 2.0)
        (`FXSystemComponent.SetFloatParameter` (`self.Number_Particles1`) "4_spawn" 2.0)
        (`FXSystemComponent.SetFloatParameter` (`self.Number_Particles4`) "4_spawn" 2.0)
        (`FXSystemComponent.SetFloatParameter` (`self.Number_Particles3`) "4_spawn" 2.0)
        (`FXSystemComponent.SetFloatParameter` (`self.Number_Particles`) "5_spawn" 2.0)
        (`FXSystemComponent.SetFloatParameter` (`self.Number_Particles1`) "5_spawn" 2.0)
        (`FXSystemComponent.SetFloatParameter` (`self.Number_Particles4`) "5_spawn" 2.0)
        (`FXSystemComponent.SetFloatParameter` (`self.Number_Particles3`) "5_spawn" 2.0)
        (`self.Velocity Numbers` _returnvalue)
        (`self.Acceleration Numbers` _returnvalue)
        (elif (<= _returnvalue_2 20)
          (`FXSystemComponent.SetFloatParameter` (`self.Number_Particles`) "0_spawn" 5.0)
          (`FXSystemComponent.SetFloatParameter` (`self.Number_Particles1`) "0_spawn" 5.0)
          (`FXSystemComponent.SetFloatParameter` (`self.Number_Particles4`) "0_spawn" 5.0)
          (`FXSystemComponent.SetFloatParameter` (`self.Number_Particles3`) "0_spawn" 5.0)
          (`FXSystemComponent.SetFloatParameter` (`self.Number_Particles`) "1_spawn" 5.0)
          (`FXSystemComponent.SetFloatParameter` (`self.Number_Particles1`) "1_spawn" 5.0)
          (`FXSystemComponent.SetFloatParameter` (`self.Number_Particles4`) "1_spawn" 5.0)
          (`FXSystemComponent.SetFloatParameter` (`self.Number_Particles3`) "1_spawn" 5.0)
          (`FXSystemComponent.SetFloatParameter` (`self.Number_Particles`) "2_spawn" 5.0)
          (`FXSystemComponent.SetFloatParameter` (`self.Number_Particles1`) "2_spawn" 5.0)
          (`FXSystemComponent.SetFloatParameter` (`self.Number_Particles4`) "2_spawn" 5.0)
          (`FXSystemComponent.SetFloatParameter` (`self.Number_Particles`) "3_spawn" 5.0)
          (`FXSystemComponent.SetFloatParameter` (`self.Number_Particles1`) "3_spawn" 5.0)
          (`FXSystemComponent.SetFloatParameter` (`self.Number_Particles4`) "3_spawn" 5.0)
          (`FXSystemComponent.SetFloatParameter` (`self.Number_Particles`) "4_spawn" 5.0)
          (`FXSystemComponent.SetFloatParameter` (`self.Number_Particles1`) "4_spawn" 5.0)
          (`FXSystemComponent.SetFloatParameter` (`self.Number_Particles4`) "4_spawn" 5.0)
          (`FXSystemComponent.SetFloatParameter` (`self.Number_Particles3`) "4_spawn" 5.0)
          (`FXSystemComponent.SetFloatParameter` (`self.Number_Particles`) "5_spawn" 5.0)
          (`FXSystemComponent.SetFloatParameter` (`self.Number_Particles1`) "5_spawn" 5.0)
          (`FXSystemComponent.SetFloatParameter` (`self.Number_Particles4`) "5_spawn" 5.0)
          (`FXSystemComponent.SetFloatParameter` (`self.Number_Particles3`) "5_spawn" 5.0)
          (`self.Velocity Numbers` _returnvalue)
          (`self.Acceleration Numbers` _returnvalue)
          (elif (> _returnvalue_2 22)
            (`FXSystemComponent.SetFloatParameter` (`self.Number_Particles`) "0_spawn" _returnvalue_3)
            (`FXSystemComponent.SetFloatParameter` (`self.Number_Particles1`) "0_spawn" _returnvalue_3)
            (`FXSystemComponent.SetFloatParameter` (`self.Number_Particles4`) "0_spawn" _returnvalue_3)
            (`FXSystemComponent.SetFloatParameter` (`self.Number_Particles3`) "0_spawn" _returnvalue_3)
            (`FXSystemComponent.SetFloatParameter` (`self.Number_Particles`) "1_spawn" _returnvalue_3)
            (`FXSystemComponent.SetFloatParameter` (`self.Number_Particles1`) "1_spawn" _returnvalue_3)
            (`FXSystemComponent.SetFloatParameter` (`self.Number_Particles4`) "1_spawn" _returnvalue_3)
            (`FXSystemComponent.SetFloatParameter` (`self.Number_Particles3`) "1_spawn" _returnvalue_3)
            (`FXSystemComponent.SetFloatParameter` (`self.Number_Particles`) "2_spawn" _returnvalue_3)
            (`FXSystemComponent.SetFloatParameter` (`self.Number_Particles1`) "2_spawn" _returnvalue_3)
            (`FXSystemComponent.SetFloatParameter` (`self.Number_Particles4`) "2_spawn" _returnvalue_3)
            (`FXSystemComponent.SetFloatParameter` (`self.Number_Particles`) "3_spawn" _returnvalue_3)
            (`FXSystemComponent.SetFloatParameter` (`self.Number_Particles1`) "3_spawn" _returnvalue_3)
            (`FXSystemComponent.SetFloatParameter` (`self.Number_Particles4`) "3_spawn" _returnvalue_3)
            (`FXSystemComponent.SetFloatParameter` (`self.Number_Particles`) "4_spawn" _returnvalue_3)
            (`FXSystemComponent.SetFloatParameter` (`self.Number_Particles1`) "4_spawn" _returnvalue_3)
            (`FXSystemComponent.SetFloatParameter` (`self.Number_Particles4`) "4_spawn" _returnvalue_3)
            (`FXSystemComponent.SetFloatParameter` (`self.Number_Particles3`) "4_spawn" _returnvalue_3)
            (`FXSystemComponent.SetFloatParameter` (`self.Number_Particles`) "5_spawn" _returnvalue_3)
            (`FXSystemComponent.SetFloatParameter` (`self.Number_Particles1`) "5_spawn" _returnvalue_3)
            (`FXSystemComponent.SetFloatParameter` (`self.Number_Particles4`) "5_spawn" _returnvalue_3)
            (`FXSystemComponent.SetFloatParameter` (`self.Number_Particles3`) "5_spawn" _returnvalue_3)
            (`self.Velocity Numbers` _returnvalue)
            (`self.Acceleration Numbers` _returnvalue)))))))

(fn `UserConstructionScript`)

(fn `Velocity Numbers`
  (params (note_freq :type "Float (double-precision)"))
  (bind _returnvalue (`KismetMathLibrary.MakeVector` (`KismetMathLibrary.RandomFloatInRange` -20.0 20.0) 45.0 note_freq))
  (bind _returnvalue_2 (`KismetMathLibrary.MakeVector` (`KismetMathLibrary.RandomFloatInRange` -50.0 50.0) 70.0 (`KismetMathLibrary.RandomFloatInRange` 0.0)))
  (bind _returnvalue_3 (`KismetMathLibrary.MakeVector` (`KismetMathLibrary.RandomFloatInRange` -5.0 5.0) 30.0))
  (if (<= note_freq 10.0)
    (`FXSystemComponent.SetVectorParameter` (`self.Number_Particles`) "0_vel" _returnvalue_3)
    (`FXSystemComponent.SetVectorParameter` (`self.Number_Particles1`) "0_vel" _returnvalue_3)
    (`FXSystemComponent.SetVectorParameter` (`self.Number_Particles4`) "0_vel" _returnvalue_3)
    (`FXSystemComponent.SetVectorParameter` (`self.Number_Particles3`) "0_vel" _returnvalue_3)
    (`FXSystemComponent.SetVectorParameter` (`self.Number_Particles2`) "0_vel" _returnvalue_3)
    (`FXSystemComponent.SetVectorParameter` (`self.Number_Particles`) "1_vel" _returnvalue_3)
    (`FXSystemComponent.SetVectorParameter` (`self.Number_Particles1`) "1_vel" _returnvalue_3)
    (`FXSystemComponent.SetVectorParameter` (`self.Number_Particles4`) "1_vel" _returnvalue_3)
    (`FXSystemComponent.SetVectorParameter` (`self.Number_Particles3`) "1_vel" _returnvalue_3)
    (`FXSystemComponent.SetVectorParameter` (`self.Number_Particles2`) "1_vel" _returnvalue_3)
    (`FXSystemComponent.SetVectorParameter` (`self.Number_Particles`) "2_vel" _returnvalue_3)
    (`FXSystemComponent.SetVectorParameter` (`self.Number_Particles1`) "2_vel" _returnvalue_3)
    (`FXSystemComponent.SetVectorParameter` (`self.Number_Particles4`) "2_vel" _returnvalue_3)
    (`FXSystemComponent.SetVectorParameter` (`self.Number_Particles3`) "2_vel" _returnvalue_3)
    (`FXSystemComponent.SetVectorParameter` (`self.Number_Particles2`) "2_vel" _returnvalue_3)
    (`FXSystemComponent.SetVectorParameter` (`self.Number_Particles`) "3_vel" _returnvalue_3)
    (`FXSystemComponent.SetVectorParameter` (`self.Number_Particles1`) "3_vel" _returnvalue_3)
    (`FXSystemComponent.SetVectorParameter` (`self.Number_Particles4`) "3_vel" _returnvalue_3)
    (`FXSystemComponent.SetVectorParameter` (`self.Number_Particles3`) "3_vel" _returnvalue_3)
    (`FXSystemComponent.SetVectorParameter` (`self.Number_Particles2`) "3_vel" _returnvalue_3)
    (`FXSystemComponent.SetVectorParameter` (`self.Number_Particles`) "4_vel" _returnvalue_3)
    (`FXSystemComponent.SetVectorParameter` (`self.Number_Particles1`) "4_vel" _returnvalue_3)
    (`FXSystemComponent.SetVectorParameter` (`self.Number_Particles4`) "4_vel" _returnvalue_3)
    (`FXSystemComponent.SetVectorParameter` (`self.Number_Particles3`) "4_vel" _returnvalue_3)
    (`FXSystemComponent.SetVectorParameter` (`self.Number_Particles2`) "4_vel" _returnvalue_3)
    (`FXSystemComponent.SetVectorParameter` (`self.Number_Particles`) "5_vel" _returnvalue_3)
    (`FXSystemComponent.SetVectorParameter` (`self.Number_Particles1`) "5_vel" _returnvalue_3)
    (`FXSystemComponent.SetVectorParameter` (`self.Number_Particles4`) "5_vel" _returnvalue_3)
    (`FXSystemComponent.SetVectorParameter` (`self.Number_Particles3`) "5_vel" _returnvalue_3)
    (`FXSystemComponent.SetVectorParameter` (`self.Number_Particles2`) "5_vel" _returnvalue_3)
    (elif (<= note_freq 20.0)
      (`FXSystemComponent.SetVectorParameter` (`self.Number_Particles`) "0_vel" _returnvalue)
      (`FXSystemComponent.SetVectorParameter` (`self.Number_Particles1`) "0_vel" _returnvalue)
      (`FXSystemComponent.SetVectorParameter` (`self.Number_Particles4`) "0_vel" _returnvalue)
      (`FXSystemComponent.SetVectorParameter` (`self.Number_Particles3`) "0_vel" _returnvalue)
      (`FXSystemComponent.SetVectorParameter` (`self.Number_Particles2`) "0_vel" _returnvalue)
      (`FXSystemComponent.SetVectorParameter` (`self.Number_Particles`) "1_vel" _returnvalue)
      (`FXSystemComponent.SetVectorParameter` (`self.Number_Particles1`) "1_vel" _returnvalue)
      (`FXSystemComponent.SetVectorParameter` (`self.Number_Particles4`) "1_vel" _returnvalue)
      (`FXSystemComponent.SetVectorParameter` (`self.Number_Particles3`) "1_vel" _returnvalue)
      (`FXSystemComponent.SetVectorParameter` (`self.Number_Particles2`) "1_vel" _returnvalue)
      (`FXSystemComponent.SetVectorParameter` (`self.Number_Particles`) "2_vel" _returnvalue)
      (`FXSystemComponent.SetVectorParameter` (`self.Number_Particles1`) "2_vel" _returnvalue)
      (`FXSystemComponent.SetVectorParameter` (`self.Number_Particles4`) "2_vel" _returnvalue)
      (`FXSystemComponent.SetVectorParameter` (`self.Number_Particles3`) "2_vel" _returnvalue)
      (`FXSystemComponent.SetVectorParameter` (`self.Number_Particles2`) "2_vel" _returnvalue)
      (`FXSystemComponent.SetVectorParameter` (`self.Number_Particles`) "3_vel" _returnvalue)
      (`FXSystemComponent.SetVectorParameter` (`self.Number_Particles1`) "3_vel" _returnvalue)
      (`FXSystemComponent.SetVectorParameter` (`self.Number_Particles4`) "3_vel" _returnvalue)
      (`FXSystemComponent.SetVectorParameter` (`self.Number_Particles3`) "3_vel" _returnvalue)
      (`FXSystemComponent.SetVectorParameter` (`self.Number_Particles2`) "3_vel" _returnvalue)
      (`FXSystemComponent.SetVectorParameter` (`self.Number_Particles`) "4_vel" _returnvalue)
      (`FXSystemComponent.SetVectorParameter` (`self.Number_Particles1`) "4_vel" _returnvalue)
      (`FXSystemComponent.SetVectorParameter` (`self.Number_Particles4`) "4_vel" _returnvalue)
      (`FXSystemComponent.SetVectorParameter` (`self.Number_Particles3`) "4_vel" _returnvalue)
      (`FXSystemComponent.SetVectorParameter` (`self.Number_Particles2`) "4_vel" _returnvalue)
      (`FXSystemComponent.SetVectorParameter` (`self.Number_Particles`) "5_vel" _returnvalue)
      (`FXSystemComponent.SetVectorParameter` (`self.Number_Particles1`) "5_vel" _returnvalue)
      (`FXSystemComponent.SetVectorParameter` (`self.Number_Particles4`) "5_vel" _returnvalue)
      (`FXSystemComponent.SetVectorParameter` (`self.Number_Particles3`) "5_vel" _returnvalue)
      (`FXSystemComponent.SetVectorParameter` (`self.Number_Particles2`) "5_vel" _returnvalue)
      (elif (> note_freq 20.0)
        (`FXSystemComponent.SetVectorParameter` (`self.Number_Particles`) "0_vel" _returnvalue_2)
        (`FXSystemComponent.SetVectorParameter` (`self.Number_Particles1`) "0_vel" _returnvalue_2)
        (`FXSystemComponent.SetVectorParameter` (`self.Number_Particles4`) "0_vel" _returnvalue_2)
        (`FXSystemComponent.SetVectorParameter` (`self.Number_Particles3`) "0_vel" _returnvalue_2)
        (`FXSystemComponent.SetVectorParameter` (`self.Number_Particles2`) "0_vel" _returnvalue_2)
        (`FXSystemComponent.SetVectorParameter` (`self.Number_Particles`) "1_vel" _returnvalue_2)
        (`FXSystemComponent.SetVectorParameter` (`self.Number_Particles1`) "1_vel" _returnvalue_2)
        (`FXSystemComponent.SetVectorParameter` (`self.Number_Particles4`) "1_vel" _returnvalue_2)
        (`FXSystemComponent.SetVectorParameter` (`self.Number_Particles3`) "1_vel" _returnvalue_2)
        (`FXSystemComponent.SetVectorParameter` (`self.Number_Particles2`) "1_vel" _returnvalue_2)
        (`FXSystemComponent.SetVectorParameter` (`self.Number_Particles`) "2_vel" _returnvalue_2)
        (`FXSystemComponent.SetVectorParameter` (`self.Number_Particles1`) "2_vel" _returnvalue_2)
        (`FXSystemComponent.SetVectorParameter` (`self.Number_Particles4`) "2_vel" _returnvalue_2)
        (`FXSystemComponent.SetVectorParameter` (`self.Number_Particles3`) "2_vel" _returnvalue_2)
        (`FXSystemComponent.SetVectorParameter` (`self.Number_Particles2`) "2_vel" _returnvalue_2)
        (`FXSystemComponent.SetVectorParameter` (`self.Number_Particles`) "3_vel" _returnvalue_2)
        (`FXSystemComponent.SetVectorParameter` (`self.Number_Particles1`) "3_vel" _returnvalue_2)
        (`FXSystemComponent.SetVectorParameter` (`self.Number_Particles4`) "3_vel" _returnvalue_2)
        (`FXSystemComponent.SetVectorParameter` (`self.Number_Particles3`) "3_vel" _returnvalue_2)
        (`FXSystemComponent.SetVectorParameter` (`self.Number_Particles2`) "3_vel" _returnvalue_2)
        (`FXSystemComponent.SetVectorParameter` (`self.Number_Particles`) "4_vel" _returnvalue_2)
        (`FXSystemComponent.SetVectorParameter` (`self.Number_Particles1`) "4_vel" _returnvalue_2)
        (`FXSystemComponent.SetVectorParameter` (`self.Number_Particles4`) "4_vel" _returnvalue_2)
        (`FXSystemComponent.SetVectorParameter` (`self.Number_Particles3`) "4_vel" _returnvalue_2)
        (`FXSystemComponent.SetVectorParameter` (`self.Number_Particles2`) "4_vel" _returnvalue_2)
        (`FXSystemComponent.SetVectorParameter` (`self.Number_Particles`) "5_vel" _returnvalue_2)
        (`FXSystemComponent.SetVectorParameter` (`self.Number_Particles1`) "5_vel" _returnvalue_2)
        (`FXSystemComponent.SetVectorParameter` (`self.Number_Particles4`) "5_vel" _returnvalue_2)
        (`FXSystemComponent.SetVectorParameter` (`self.Number_Particles3`) "5_vel" _returnvalue_2)
        (`FXSystemComponent.SetVectorParameter` (`self.Number_Particles2`) "5_vel" _returnvalue_2)))))