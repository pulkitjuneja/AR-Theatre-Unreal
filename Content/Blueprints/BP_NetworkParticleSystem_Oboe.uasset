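; Networked oboe particle actor that drives magic circle and bubble effects from incoming OSC messages.
; On the server it opens an OSC listener at the game instance's machine IP.
; "P" addresses pass a float frequency that scales disc dots, one of three rings in rotation, and four bubble systems; the flies effect is an empty stub.
; "S" addresses trigger ServerTravel to the Madeleine_Dring map.
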(event `self.ReceiveBeginPlay`
  (bind _asbp_game_instace (cast `/Game/Blueprints/BP_GameInstace` (`GameplayStatics.GetGameInstance`)))
  (if (`/Game/Blueprints/BP_GameInstace.isServer` _asbp_game_instace)
    (`KismetSystemLibrary.PrintString` "Creating osc server")
    (bind _returnvalue (`OSCManager.CreateOSCServer` (`/Game/Blueprints/BP_GameInstace.MachineIP` _asbp_game_instace) 7000 false true "" null))
    (`KismetSystemLibrary.PrintString` "OSC server created")
    (bind _output_get (set `self.OscServer` _returnvalue))
    (clear `OSCServer.OnOscBundleReceived` _output_get)
    (add `OSCServer.OnOscMessageReceived` _output_get (`|CreateDelegate` :!event `OSCMessageReceived`))))

(event `OSCMessageReceived`
  (params (Message :type "OSCMessage Structure (by ref)") (IPAddress :type String) (Port :type Integer))
  (bind _returnvalue (`OSCManager.GetOSCMessageAddress` Message))
  (bind _returnvalue_2 (`OSCManager.GetOSCAddressFullPath` _returnvalue))
  (`|ExecutionSequence`
    (:`then_0`
      (bind _returnvalue_3 (`KismetStringLibrary.GetSubstring` _returnvalue_2 1))
      (if (`KismetStringLibrary.EqualEqual_StrStr` _returnvalue_3 "P")
        (bind _value (`OSCManager.GetFloat` Message))
        (`self.Spawn Effects` _value)))
    (:`then_1`
      (if (`KismetStringLibrary.EqualEqual_StrStr` _returnvalue_3 "S")
        (`KismetSystemLibrary.PrintString` "Switching")
        (`KismetSystemLibrary.ExecuteConsoleCommand` "ServerTravel Madeleine_Dring" null)))))

(event `Spawn Effects`
  (params (Frequency :type "Float (double-precision)"))
  (`self.Spawn Oboe Effects` (* Frequency 1.0)))

(fn `Spawn Oboe Effects`
  (params (Frequency :type "Float (double-precision)"))
  (`|ExecutionSequence`
    (:`then_0`
      (`self.spawn_disc` Frequency))
    (:`then_1`
      (`self.spawn_flies` Frequency))
    (:`then_2`
      (`self.spawn_bubbles` Frequency))))

(fn `spawn_bubbles`
  (params (frequency :type "Float (double-precision)"))
  (bind _returnvalue (* frequency 100.0))
  (if (`KismetMathLibrary.Conv_IntToBool` (`KismetMathLibrary.Round` _returnvalue))
    (`FXSystemComponent.SetFloatParameter` (`self.Bubbles`) "spawn_bubble" _returnvalue)
    (`FXSystemComponent.SetFloatParameter` (`self.Bubbles3`) "spawn_bubble" _returnvalue)
    (`FXSystemComponent.SetFloatParameter` (`self.Bubbles2`) "spawn_bubble" _returnvalue)
    (`FXSystemComponent.SetFloatParameter` (`self.Bubbles1`) "spawn_bubble" _returnvalue)
    (else
      (`FXSystemComponent.SetFloatParameter` (`self.Bubbles`) "spawn_bubble" 0.0)
      (`FXSystemComponent.SetFloatParameter` (`self.Bubbles3`) "spawn_bubble" 0.0)
      (`FXSystemComponent.SetFloatParameter` (`self.Bubbles2`) "spawn_bubble" 0.0)
      (`FXSystemComponent.SetFloatParameter` (`self.Bubbles1`) "spawn_bubble" 0.0))))

(fn `spawn_disc`
  (params (frequency :type "Float (double-precision)"))
  (bind _returnvalue (* frequency 200.0))
  (bind _magiccircle (`self.MagicCircle`))
  (if (>= frequency 0.0)
    (`|ExecutionSequence`
      (:`then_0`
        (`FXSystemComponent.SetFloatParameter` (`self.MagicCircle`) "dot_spawn_count" (+ (* frequency 100.0) 20.0)))
      (:`then_1`
        (`|ExecutionSequence`
          (:`then_0`
            (switch `int` (`self.Counter`)
              (:`0`
                (`FXSystemComponent.SetFloatParameter` _magiccircle "ring_size" _returnvalue))
              (:`1`
                (`FXSystemComponent.SetFloatParameter` _magiccircle "ring_size_1" _returnvalue))
              (:`2`
                (`FXSystemComponent.SetFloatParameter` _magiccircle "ring_size_2" _returnvalue))))
          (:`then_1`
            (bind _result (`/Engine/EditorBlueprintResources/StandardMacros.IncrementInt` (`self.Counter`))
              (:`  `
                (bind _output_get (set `self.Counter` _result))
                (if (>= _output_get 3)
                  (set `self.Counter` 0))))))))))

(fn `spawn_flies`
  (params (frequency :type "Float (double-precision)")))

(fn `UserConstructionScript`)