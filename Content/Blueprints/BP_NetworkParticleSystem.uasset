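; Actor that drives leaf, wind, swirl and music-note particle effects from a value received over OSC.
; On the server only, BeginPlay opens an OSC server on the game instance's machine IP and binds a message handler.
; "P" addresses feed a frequency into Spawn functions that set particle parameters by linear scaling or thresholds, with randomized note velocity and acceleration.
; "S" addresses trigger ServerTravel to Alien_09.
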(event `self.ReceiveBeginPlay`
  (bind _asbp_game_instace (cast `/Game/Blueprints/BP_GameInstace` (`GameplayStatics.GetGameInstance`)))
  (if (`/Game/Blueprints/BP_GameInstace.isServer` _asbp_game_instace)
    (`KismetSystemLibrary.PrintString` "Creating osc server")
    (bind _returnvalue (`OSCManager.CreateOSCServer` (`/Game/Blueprints/BP_GameInstace.MachineIP` _asbp_game_instace) 7000 false true "" null))
    (`KismetSystemLibrary.PrintString` "OSC server created")
    (bind _output_get (set `self.OscServer` _returnvalue))
    (clear `OSCServer.OnOscBundleReceived` _output_get)
    (add `OSCServer.OnOscMessageReceived` _output_get (`|CreateDelegate` :!event `OSCMessageReceived`))))

(event `OSCMessageReceived`
  (params (Message :type "OSCMessage Structure (by ref)") (IPAddress :type String) (Port :type Integer))
  (bind _returnvalue (`OSCManager.GetOSCMessageAddress` Message))
  (bind _returnvalue_2 (`OSCManager.GetOSCAddressFullPath` _returnvalue))
  (`|ExecutionSequence`
    (:`then_0`
      (bind _returnvalue_3 (`KismetStringLibrary.GetSubstring` _returnvalue_2 1))
      (if (`KismetStringLibrary.EqualEqual_StrStr` _returnvalue_3 "P")
        (bind _value (`OSCManager.GetFloat` Message))
        (`self.Spawn Effects` _value)))
    (:`then_1`
      (if (`KismetStringLibrary.EqualEqual_StrStr` _returnvalue_3 "S")
        (`KismetSystemLibrary.PrintString` "Switching")
        (`KismetSystemLibrary.ExecuteConsoleCommand` "ServerTravel Alien_09" null)))))

(event `Spawn Effects`
  (params (Frequency :type "Float (double-precision)"))
  (bind _returnvalue (* Frequency 1.0))
  (`self.SpawnLeafFunction` _returnvalue)
  (`self.SpawnWindFunction` _returnvalue)
  (`self.SpawnWindSwirls` _returnvalue)
  (`self.Spawn Notes` _returnvalue))

(fn `AccelerationNotes`
  (params (freq_notes_acc :type "Float (double-precision)"))
  (bind _returnvalue (`KismetMathLibrary.MakeVector` (`KismetMathLibrary.RandomFloatInRange` -2.0 2.0) 0.0 freq_notes_acc))
  (bind _returnvalue_2 (`KismetMathLibrary.MakeVector` (`KismetMathLibrary.RandomFloatInRange` -10.0 10.0) 5.0 (`KismetMathLibrary.RandomFloatInRange` 0.0 15.0)))
  (bind _returnvalue_3 (`KismetMathLibrary.MakeVector` (`KismetMathLibrary.RandomFloatInRange` -6.0 6.0) 0.0 freq_notes_acc))
  (if (<= freq_notes_acc 10.0)
    (`FXSystemComponent.SetVectorParameter` (`self.note_particles`) "eighth_acc" _returnvalue)
    (`FXSystemComponent.SetVectorParameter` (`self.Note_Particles2`) "eighth_acc" _returnvalue)
    (`FXSystemComponent.SetVectorParameter` (`self.Note_Particles1`) "eighth_acc" _returnvalue)
    (`FXSystemComponent.SetVectorParameter` (`self.note_particles`) "half_acc" _returnvalue)
    (`FXSystemComponent.SetVectorParameter` (`self.Note_Particles2`) "half_acc" _returnvalue)
    (`FXSystemComponent.SetVectorParameter` (`self.Note_Particles1`) "half_acc" _returnvalue)
    (`FXSystemComponent.SetVectorParameter` (`self.note_particles`) "sixteenth_acc" _returnvalue)
    (`FXSystemComponent.SetVectorParameter` (`self.Note_Particles2`) "sixteenth_acc" _returnvalue)
    (`FXSystemComponent.SetVectorParameter` (`self.Note_Particles1`) "sixteenth_acc" _returnvalue)
    (elif (<= freq_notes_acc 20.0)
      (`FXSystemComponent.SetVectorParameter` (`self.note_particles`) "eighth_acc" _returnvalue_3)
      (`FXSystemComponent.SetVectorParameter` (`self.Note_Particles2`) "eighth_acc" _returnvalue_3)
      (`FXSystemComponent.SetVectorParameter` (`self.Note_Particles1`) "eighth_acc" _returnvalue_3)
      (`FXSystemComponent.SetVectorParameter` (`self.note_particles`) "half_acc" _returnvalue_3)
      (`FXSystemComponent.SetVectorParameter` (`self.Note_Particles2`) "half_acc" _returnvalue_3)
      (`FXSystemComponent.SetVectorParameter` (`self.Note_Particles1`) "half_acc" _returnvalue_3)
      (`FXSystemComponent.SetVectorParameter` (`self.note_particles`) "sixteenth_acc" _returnvalue_3)
      (`FXSystemComponent.SetVectorParameter` (`self.Note_Particles2`) "sixteenth_acc" _returnvalue_3)
      (`FXSystemComponent.SetVectorParameter` (`self.Note_Particles1`) "sixteenth_acc" _returnvalue_3)
      (elif (> freq_notes_acc 20.0)
        (`FXSystemComponent.SetVectorParameter` (`self.note_particles`) "eighth_acc" _returnvalue_2)
        (`FXSystemComponent.SetVectorParameter` (`self.Note_Particles2`) "eighth_acc" _returnvalue_2)
        (`FXSystemComponent.SetVectorParameter` (`self.Note_Particles1`) "eighth_acc" _returnvalue_2)
        (`FXSystemComponent.SetVectorParameter` (`self.note_particles`) "half_acc" _returnvalue_2)
        (`FXSystemComponent.SetVectorParameter` (`self.Note_Particles2`) "half_acc" _returnvalue_2)
        (`FXSystemComponent.SetVectorParameter` (`self.Note_Particles1`) "half_acc" _returnvalue_2)
        (`FXSystemComponent.SetVectorParameter` (`self.note_particles`) "sixteenth_acc" _returnvalue_2)
        (`FXSystemComponent.SetVectorParameter` (`self.Note_Particles2`) "sixteenth_acc" _returnvalue_2)
        (`FXSystemComponent.SetVectorParameter` (`self.Note_Particles1`) "sixteenth_acc" _returnvalue_2)))))

(fn `PrintFrequency`
  (params (frequency :type "Float (double-precision)"))
  (bind _returnvalue (* frequency 100.0))
  (if (>= _returnvalue 1.0)
    (`KismetSystemLibrary.PrintString` (`KismetStringLibrary.Conv_IntToString` (`KismetMathLibrary.Round` _returnvalue)))))

(fn `Spawn Notes`
  (params (freq_spawn_notes :type "Float (double-precision)"))
  (bind _returnvalue (* freq_spawn_notes 100.0))
  (bind _returnvalue_2 (`KismetMathLibrary.Round` _returnvalue))
  (bind _returnvalue_3 (* _returnvalue 1.0))
  (if (< _returnvalue_2 1)
    (`FXSystemComponent.SetFloatParameter` (`self.note_particles`) "eighth_spawn" 0.0)
    (`FXSystemComponent.SetFloatParameter` (`self.Note_Particles1`) "eighth_spawn" 0.0)
    (`FXSystemComponent.SetFloatParameter` (`self.Note_Particles2`) "eighth_spawn" 0.0)
    (`FXSystemComponent.SetFloatParameter` (`self.note_particles`) "half_spawn" 0.0)
    (`FXSystemComponent.SetFloatParameter` (`self.Note_Particles2`) "half_spawn" 0.0)
    (`FXSystemComponent.SetFloatParameter` (`self.Note_Particles1`) "half_spawn" 0.0)
    (`FXSystemComponent.SetFloatParameter` (`self.note_particles`) "sixteenth_spawn" 0.0)
    (`FXSystemComponent.SetFloatParameter` (`self.Note_Particles2`) "sixteenth_spawn" 0.0)
    (`FXSystemComponent.SetFloatParameter` (`self.Note_Particles1`) "sixteenth_spawn" 0.0)
    (elif (<= _returnvalue_2 5)
      (`FXSystemComponent.SetFloatParameter` (`self.note_particles`) "eighth_spawn" 0.5)
      (`FXSystemComponent.SetFloatParameter` (`self.Note_Particles1`) "eighth_spawn" 0.5)
      (`FXSystemComponent.SetFloatParameter` (`self.Note_Particles2`) "eighth_spawn" 0.5)
      (`FXSystemComponent.SetFloatParameter` (`self.note_particles`) "half_spawn" 0.5)
      (`FXSystemComponent.SetFloatParameter` (`self.Note_Particles2`) "half_spawn" 0.5)
      (`FXSystemComponent.SetFloatParameter` (`self.Note_Particles1`) "half_spawn" 0.5)
      (`FXSystemComponent.SetFloatParameter` (`self.note_particles`) "sixteenth_spawn" 0.5)
      (`FXSystemComponent.SetFloatParameter` (`self.Note_Particles2`) "sixteenth_spawn" 0.5)
      (`FXSystemComponent.SetFloatParameter` (`self.Note_Particles1`) "sixteenth_spawn" 0.5)
      (`self.VelocityNotes` _returnvalue)
      (`self.AccelerationNotes` _returnvalue)
      (elif (<= _returnvalue_2 10)
        (`FXSystemComponent.SetFloatParameter` (`self.note_particles`) "eighth_spawn" 2.0)
        (`FXSystemComponent.SetFloatParameter` (`self.Note_Particles2`) "eighth_spawn" 2.0)
        (`FXSystemComponent.SetFloatParameter` (`self.Note_Particles1`) "eighth_spawn" 2.0)
        (`FXSystemComponent.SetFloatParameter` (`self.note_particles`) "half_spawn" 2.0)
        (`FXSystemComponent.SetFloatParameter` (`self.Note_Particles2`) "half_spawn" 2.0)
        (`FXSystemComponent.SetFloatParameter` (`self.Note_Particles1`) "half_spawn" 2.0)
        (`FXSystemComponent.SetFloatParameter` (`self.note_particles`) "sixteenth_spawn" 2.0)
        (`FXSystemComponent.SetFloatParameter` (`self.Note_Particles2`) "sixteenth_spawn" 2.0)
        (`FXSystemComponent.SetFloatParameter` (`self.Note_Particles1`) "sixteenth_spawn" 2.0)
        (`self.VelocityNotes` _returnvalue)
        (`self.AccelerationNotes` _returnvalue)
        (elif (<= _returnvalue_2 20)
          (`FXSystemComponent.SetFloatParameter` (`self.note_particles`) "eighth_spawn" 5.0)
          (`FXSystemComponent.SetFloatParameter` (`self.Note_Particles1`) "eighth_spawn" 5.0)
          (`FXSystemComponent.SetFloatParameter` (`self.Note_Particles2`) "eighth_spawn" 5.0)
          (`FXSystemComponent.SetFloatParameter` (`self.note_particles`) "half_spawn" 5.0)
          (`FXSystemComponent.SetFloatParameter` (`self.Note_Particles1`) "half_spawn" 5.0)
          (`FXSystemComponent.SetFloatParameter` (`self.Note_Particles2`) "half_spawn" 5.0)
          (`FXSystemComponent.SetFloatParameter` (`self.note_particles`) "sixteenth_spawn" 5.0)
          (`FXSystemComponent.SetFloatParameter` (`self.Note_Particles2`) "sixteenth_spawn" 5.0)
          (`FXSystemComponent.SetFloatParameter` (`self.Note_Particles1`) "sixteenth_spawn" 5.0)
          (`self.VelocityNotes` _returnvalue)
          (`self.AccelerationNotes` _returnvalue)
          (elif (> _returnvalue_2 22)
            (`FXSystemComponent.SetFloatParameter` (`self.note_particles`) "eighth_spawn" _returnvalue_3)
            (`FXSystemComponent.SetFloatParameter` (`self.Note_Particles2`) "eighth_spawn" _returnvalue_3)
            (`FXSystemComponent.SetFloatParameter` (`self.Note_Particles1`) "eighth_spawn" _returnvalue_3)
            (`FXSystemComponent.SetFloatParameter` (`self.note_particles`) "half_spawn" _returnvalue_3)
            (`FXSystemComponent.SetFloatParameter` (`self.Note_Particles2`) "half_spawn" _returnvalue_3)
            (`FXSystemComponent.SetFloatParameter` (`self.Note_Particles1`) "half_spawn" _returnvalue_3)
            (`FXSystemComponent.SetFloatParameter` (`self.note_particles`) "sixteenth_spawn" _returnvalue_3)
            (`FXSystemComponent.SetFloatParameter` (`self.Note_Particles2`) "sixteenth_spawn" _returnvalue_3)
            (`FXSystemComponent.SetFloatParameter` (`self.Note_Particles1`) "sixteenth_spawn" _returnvalue_3)
            (`self.VelocityNotes` _returnvalue)
            (`self.AccelerationNotes` _returnvalue)))))))

(fn `SpawnLeafFunction`
  (params (freq_spawn :type "Float (double-precision)"))
  (bind _returnvalue (/ (`KismetMathLibrary.Conv_IntToDouble` (`KismetMathLibrary.Round` (* freq_spawn 100.0))) 2.0))
  (`FXSystemComponent.SetFloatParameter` (`self.leaf_particles`) "leaf_spawn" _returnvalue)
  (`FXSystemComponent.SetFloatParameter` (`self.green_leaf_particles`) "green_leaf_spawn" _returnvalue))

(fn `SpawnWindFunction`
  (params (freq_spawn_wind :type "Float (double-precision)"))
  (if (>= (`KismetMathLibrary.Round` (* freq_spawn_wind 100.0)) 10)
    (`FXSystemComponent.SetFloatParameter` (`self.wind_line_particles`) "wind_point_spawn" 1.0)
    (`FXSystemComponent.SetFloatParameter` (`self.wind_line_particles`) "wind_line_spawn" 1.0)
    (else
      (`FXSystemComponent.SetFloatParameter` (`self.wind_line_particles`) "wind_point_spawn" 0.0)
      (`FXSystemComponent.SetFloatParameter` (`self.wind_line_particles`) "wind_line_spawn" 0.0))))

(fn `SpawnWindSwirls`
  (params (Frequency :type "Float (double-precision)"))
  (if (>= (`KismetMathLibrary.Round` (* Frequency 100.0)) 20)
    (`FXSystemComponent.SetFloatParameter` (`self.wind_swirls_particles`) "wind_swirl_point_spawn" 4.0)
    (`FXSystemComponent.SetFloatParameter` (`self.wind_swirls_particles`) "swirl_wind_spawn" 1.0)
    (else
      (`FXSystemComponent.SetFloatParameter` (`self.wind_swirls_particles`) "wind_swirl_point_spawn" 0.0)
      (`FXSystemComponent.SetFloatParameter` (`self.wind_swirls_particles`) "swirl_wind_spawn" 0.0))))

(fn `UserConstructionScript`)

(fn `VelocityNotes`
  (params (note_freq :type "Float (double-precision)"))
  (bind _returnvalue (`KismetMathLibrary.MakeVector` (`KismetMathLibrary.RandomFloatInRange` -20.0 20.0) 45.0))
  (bind _returnvalue_2 (`KismetMathLibrary.MakeVector` (`KismetMathLibrary.RandomFloatInRange` -50.0 50.0) 70.0 (`KismetMathLibrary.RandomFloatInRange` 0.0)))
  (bind _returnvalue_3 (`KismetMathLibrary.MakeVector` (`KismetMathLibrary.RandomFloatInRange` -5.0 5.0) 30.0))
  (if (<= note_freq 10.0)
    (`FXSystemComponent.SetVectorParameter` (`self.note_particles`) "eighth_vel" _returnvalue_3)
    (`FXSystemComponent.SetVectorParameter` (`self.Note_Particles2`) "eighth_vel" _returnvalue_3)
    (`FXSystemComponent.SetVectorParameter` (`self.Note_Particles1`) "eighth_vel" _returnvalue_3)
    (`FXSystemComponent.SetVectorParameter` (`self.note_particles`) "half_vel" _returnvalue_3)
    (`FXSystemComponent.SetVectorParameter` (`self.Note_Particles2`) "half_vel" _returnvalue_3)
    (`FXSystemComponent.SetVectorParameter` (`self.Note_Particles1`) "half_vel" _returnvalue_3)
    (`FXSystemComponent.SetVectorParameter` (`self.note_particles`) "sixteenth_vel" _returnvalue_3)
    (`FXSystemComponent.SetVectorParameter` (`self.Note_Particles2`) "sixteenth_vel" _returnvalue_3)
    (`FXSystemComponent.SetVectorParameter` (`self.Note_Particles1`) "sixteenth_vel" _returnvalue_3)
    (elif (<= note_freq 20.0)
      (`FXSystemComponent.SetVectorParameter` (`self.note_particles`) "eighth_vel" _returnvalue)
      (`FXSystemComponent.SetVectorParameter` (`self.Note_Particles2`) "eighth_vel" _returnvalue)
      (`FXSystemComponent.SetVectorParameter` (`self.Note_Particles1`) "eighth_vel" _returnvalue)
      (`FXSystemComponent.SetVectorParameter` (`self.note_particles`) "half_vel" _returnvalue)
      (`FXSystemComponent.SetVectorParameter` (`self.Note_Particles2`) "half_vel" _returnvalue)
      (`FXSystemComponent.SetVectorParameter` (`self.Note_Particles1`) "half_vel" _returnvalue)
      (`FXSystemComponent.SetVectorParameter` (`self.note_particles`) "sixteenth_vel" _returnvalue)
      (`FXSystemComponent.SetVectorParameter` (`self.Note_Particles2`) "sixteenth_vel" _returnvalue)
      (`FXSystemComponent.SetVectorParameter` (`self.Note_Particles1`) "sixteenth_vel" _returnvalue)
      (elif (> note_freq 20.0)
        (`FXSystemComponent.SetVectorParameter` (`self.note_particles`) "eighth_vel" _returnvalue_2)
        (`FXSystemComponent.SetVectorParameter` (`self.Note_Particles2`) "eighth_vel" _returnvalue_2)
        (`FXSystemComponent.SetVectorParameter` (`self.Note_Particles1`) "eighth_vel" _returnvalue_2)
        (`FXSystemComponent.SetVectorParameter` (`self.note_particles`) "half_vel" _returnvalue_2)
        (`FXSystemComponent.SetVectorParameter` (`self.Note_Particles2`) "half_vel" _returnvalue_2)
        (`FXSystemComponent.SetVectorParameter` (`self.Note_Particles1`) "half_vel" _returnvalue_2)
        (`FXSystemComponent.SetVectorParameter` (`self.note_particles`) "sixteenth_vel" _returnvalue_2)
        (`FXSystemComponent.SetVectorParameter` (`self.Note_Particles2`) "sixteenth_vel" _returnvalue_2)
        (`FXSystemComponent.SetVectorParameter` (`self.Note_Particles1`) "sixteenth_vel" _returnvalue_2)))))