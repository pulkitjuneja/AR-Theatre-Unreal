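; Networked particle actor that drives a confetti effect from incoming OSC messages.
; On BeginPlay, only when the game instance is flagged as server, it starts an OSC server on a hardcoded IP and port.
; Addresses starting with "P" pass a scaled float through thresholds into the confetti's spawn parameter.
; Addresses starting with "S" trigger a ServerTravel to the Alien_09 map.
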(event `self.ReceiveBeginPlay`
  (bind _asbp_game_instace (cast `/Game/Blueprints/BP_GameInstace` (`GameplayStatics.GetGameInstance`)))
  (if (`/Game/Blueprints/BP_GameInstace.isServer` _asbp_game_instace)
    (`KismetSystemLibrary.PrintString` "Creating osc server")
    (bind _returnvalue (`OSCManager.CreateOSCServer` "129.21.139.127" 7000 false true "" null))
    (`KismetSystemLibrary.PrintString` "OSC server created")
    (bind _output_get (set `self.OscServer` _returnvalue))
    (clear `OSCServer.OnOscBundleReceived` _output_get)
    (add `OSCServer.OnOscMessageReceived` _output_get (`|CreateDelegate` :!event `OSCMessageReceived`))))

(event `OSCMessageReceived`
  (params (Message :type "OSCMessage Structure (by ref)") (IPAddress :type String) (Port :type Integer))
  (bind _returnvalue (`OSCManager.GetOSCMessageAddress` Message))
  (bind _returnvalue_2 (`OSCManager.GetOSCAddressFullPath` _returnvalue))
  (`|ExecutionSequence`
    (:`then_0`
      (bind _returnvalue_3 (`KismetStringLibrary.GetSubstring` _returnvalue_2 1))
      (if (`KismetStringLibrary.EqualEqual_StrStr` _returnvalue_3 "P")
        (bind _value (`OSCManager.GetFloat` Message))
        (`self.Spawn Effects` _value)))
    (:`then_1`
      (if (`KismetStringLibrary.EqualEqual_StrStr` _returnvalue_3 "S")
        (`KismetSystemLibrary.PrintString` "Switching")
        (`KismetSystemLibrary.ExecuteConsoleCommand` "ServerTravel Alien_09" null)))))

(event `Spawn Effects`
  (params (Frequency :type "Float (double-precision)"))
  (`|ExecutionSequence`
    (:`then_0`
      (`KismetSystemLibrary.PrintString` (`KismetStringLibrary.Conv_DoubleToString` (* Frequency 100.0))))
    (:`then_1`
      (`self.Spawn Confetti` (* Frequency 10.0)))))

(fn `PrintFrequency`
  (params (frequency :type "Float (double-precision)"))
  (bind _returnvalue (* frequency 100.0))
  (if (>= _returnvalue 1.0)
    (`KismetSystemLibrary.PrintString` (`KismetStringLibrary.Conv_IntToString` (`KismetMathLibrary.Round` _returnvalue)))))

(fn `Spawn Confetti`
  (params (Frequency :type "Float (double-precision)"))
  (bind _returnvalue (* Frequency 100.0))
  (if (>= Frequency 1.0)
    (if (>= _returnvalue 10.0)
      (`FXSystemComponent.SetFloatParameter` (`self.confetti`) "generate_confetti" _returnvalue))))

(fn `UserConstructionScript`)