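; BP_Particles is a Blueprint that switches wind particle effects on or off according to a frequency value passed in.
; The WindParticles event forwards Frequency to SpawnWind, which scales it by 100, rounds it and compares it to a threshold.
; The result sets the point and line spawn float parameters on the Wind particle component together, as either fully on or off.
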(event `WindParticles`
  (params (frequency :type "Float (double-precision)"))
  (`self.SpawnWind` frequency))

(fn `SpawnWind`
  (params (Frequency :type "Float (double-precision)"))
  (bind _wind (`self.Wind`))
  (if (>= (`KismetMathLibrary.Round` (* Frequency 100.0)) 4)
    (`FXSystemComponent.SetFloatParameter` _wind "wind_point_spawn" 1.0)
    (`FXSystemComponent.SetFloatParameter` _wind "wind_line_spawn" 1.0)
    (else
      (`FXSystemComponent.SetFloatParameter` _wind "wind_point_spawn" 0.0)
      (`FXSystemComponent.SetFloatParameter` _wind "wind_line_spawn" 0.0))))

(fn `UserConstructionScript`)