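; BP_Magic_Circle is an oboe effect Blueprint that drives magic circle particles from OSC messages.
; Each message's first float, treated as frequency, scales the dot spawn count and one ring size.
; A cycling three-step counter picks the ring, with two steps targeting ring one and one targeting ring two.
; Tick forces both firefly colors to black, and the firefly spawn function is an empty stub.
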(event `OSCMessageReceived`
  (params (Message :type "OSCMessage Structure (by ref)") (IPAddress :type String) (Port :type Integer))
  (bind _returnvalue (`OSCManager.GetOSCMessageAddress` Message))
  (`OSCManager.GetOSCAddressFullPath` _returnvalue)
  (bind _value (`OSCManager.GetFloat` Message))
  (`self.Spawn Effects` _value))

(event `self.ReceiveBeginPlay`)

(event `self.ReceiveTick`
  (params (DeltaSeconds :type "Float (single-precision)"))
  (bind _firefly_changing (`self.firefly_changing`))
  (`|ExecutionSequence`
    (:`then_0`
      (`FXSystemComponent.SetColorParameter` :`self` _firefly_changing :`ParameterName` "Color1"))
    (:`then_1`
      (`FXSystemComponent.SetColorParameter` :`self` _firefly_changing :`ParameterName` "Color2"))))

(fn `Spawn Effects`
  (params (Frequency :type "Float (double-precision)"))
  (`|ExecutionSequence`
    (:`then_0`
      (`self.spawn_disc` Frequency))
    (:`then_1`
      (`self.spawn_flies` Frequency))))

(fn `spawn_disc`
  (params (frequency :type "Float (double-precision)"))
  (bind _returnvalue (* frequency 200.0))
  (if (>= frequency frequency)
    (`|ExecutionSequence`
      (:`then_0`
        (`FXSystemComponent.SetFloatParameter` (`self.P_MagicCircle1`) "dot_spawn_count" (+ (* frequency 100.0) 20.0)))
      (:`then_1`
        (`|ExecutionSequence`
          (:`then_0`
            (switch `int` (`self.counter`)
              (:`0`
                (`FXSystemComponent.SetFloatParameter` (`self.P_MagicCircle1`) "ring_size_1" _returnvalue))
              (:`1`
                (`FXSystemComponent.SetFloatParameter` (`self.P_MagicCircle1`) "ring_size_1" _returnvalue))
              (:`2`
                (`FXSystemComponent.SetFloatParameter` (`self.P_MagicCircle1`) "ring_size_2" _returnvalue))))
          (:`then_1`
            (bind _result (`/Engine/EditorBlueprintResources/StandardMacros.IncrementInt` (`self.counter`))
              (:`  `
                (bind _output_get (set `self.counter` _result))
                (if (>= _output_get 3)
                  (set `self.counter` 0))))))))))

(fn `spawn_flies`
  (params (frequency :type "Float (double-precision)")))

(fn `UserConstructionScript`)