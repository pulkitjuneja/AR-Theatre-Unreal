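; BP_Magic_Circle is a magic circle particle effect Blueprint with an OSC message handler.
; The handler passes the message's first float to SpawnEffects, which calls SpawnDisc and an empty SpawnFlies stub with a fixed zero instead.
; SpawnDisc derives the particle's dot spawn count and ring size from its input, so both currently receive constant values.
; The OSC address is read but never used.
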(event `OSCMessageReceived`
  (params (Message :type "OSCMessage Structure (by ref)") (IPAddress :type String) (Port :type Integer))
  (bind _returnvalue (`OSCManager.GetOSCMessageAddress` Message))
  (`OSCManager.GetOSCAddressFullPath` _returnvalue)
  (bind _value (`OSCManager.GetFloat` Message))
  (`self.Spawn Effects` _value))

(event `self.ReceiveBeginPlay`)

(fn `Spawn Effects`
  (params (Frequency :type "Float (double-precision)"))
  (`|ExecutionSequence`
    (:`then_0`
      (`self.spawn_disc` 0.0))
    (:`then_1`
      (`self.spawn_flies` 0.0))))

(fn `spawn_disc`
  (params (frequency :type "Float (double-precision)"))
  (bind _p_magiccircle1 (`self.P_MagicCircle1`))
  (`|ExecutionSequence`
    (:`then_0`
      (`FXSystemComponent.SetFloatParameter` _p_magiccircle1 "dot_spawn_count" (+ (* frequency 100.0) 20.0)))
    (:`then_1`
      (`FXSystemComponent.SetFloatParameter` _p_magiccircle1 "ring_size" (* frequency 200.0)))))

(fn `spawn_flies`
  (params (frequency :type "Float (double-precision)")))

(fn `UserConstructionScript`)