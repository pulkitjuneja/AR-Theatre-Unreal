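; Audio-reactive actor that drives leaf, wind and music note particle effects from captured audio, apparently microphone input.
; Each Tick it reads the first value of an AudioManager linear spectrum, scales it by 100 and prints it when at least one.
; Leaf spawn scales with that level, while wind lines and swirls switch on at thresholds.
; Note spawn rate, randomized velocity and acceleration change in tiers as the level rises.
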(event `self.ReceiveBeginPlay`
  (bind _returnvalue (`|GenericCreateObject` null self))
  (set `self.AudioManager` null _returnvalue)
  (bind _returnvalue_2 (`self.InitCapturerAudio` (`.AudioManager` (`self.AudioManager`))))
  (if _returnvalue_2
    (`self.InitSpectrumConfig` (`.AudioManager` (`self.AudioManager`)) 0 0 0 1 0.02 30 true 1)
    (`self.InitAmplitudeConfig` (`.AudioManager` (`self.AudioManager`)) 0 0 1 0.02)
    (`self.StartCapture` (`.AudioManager` (`self.AudioManager`)) false false)
    (else
      (`KismetSystemLibrary.PrintString` "Sound Not Being Captured. Please Check Microphone."))))

(event `self.ReceiveTick`
  (params (DeltaSeconds :type "Float (single-precision)"))
  (if (`MagicLeapCameraFunctionLibrary.IsCapturing` (`.AudioManager` (`self.AudioManager`)))
    (bind _frequencies (`self.GetSpectrum` (`.AudioManager` (`self.AudioManager`)) false))
    (bind _output (`|GetArrayItem` _frequencies))
    (`self.SpawnLeafFunction` _output)
    (`self.SpawnWindFunction` _output)
    (`self.SpawnWindSwirls` _output)
    (`self.Spawn Notes` _output)
    (`self.PrintFrequency` _output)))

(fn `AccelerationNotes`
  (params (freq_notes_acc :type "Float (double-precision)"))
  (bind _returnvalue (`KismetMathLibrary.MakeVector` (`KismetMathLibrary.RandomFloatInRange` -2.0 2.0) 0.0 freq_notes_acc))
  (bind _returnvalue_2 (`KismetMathLibrary.MakeVector` (`KismetMathLibrary.RandomFloatInRange` -10.0 10.0) 5.0 (`KismetMathLibrary.RandomFloatInRange` 0.0 15.0)))
  (bind _returnvalue_3 (`KismetMathLibrary.MakeVector` (`KismetMathLibrary.RandomFloatInRange` -6.0 6.0) 0.0 freq_notes_acc))
  (if (<= freq_notes_acc 10.0)
    (`FXSystemComponent.SetVectorParameter` (`self.note_particles`) "eighth_acc" _returnvalue)
    (`FXSystemComponent.SetVectorParameter` (`self.note_particles`) "half_acc" _returnvalue)
    (`FXSystemComponent.SetVectorParameter` (`self.note_particles`) "sixteenth_acc" _returnvalue)
    (elif (<= freq_notes_acc 20.0)
      (`FXSystemComponent.SetVectorParameter` (`self.note_particles`) "eighth_acc" _returnvalue_3)
      (`FXSystemComponent.SetVectorParameter` (`self.note_particles`) "half_acc" _returnvalue_3)
      (`FXSystemComponent.SetVectorParameter` (`self.note_particles`) "sixteenth_acc" _returnvalue_3)
      (elif (> freq_notes_acc 20.0)
        (`FXSystemComponent.SetVectorParameter` (`self.note_particles`) "eighth_acc" _returnvalue_2)
        (`FXSystemComponent.SetVectorParameter` (`self.note_particles`) "half_acc" _returnvalue_2)
        (`FXSystemComponent.SetVectorParameter` (`self.note_particles`) "sixteenth_acc" _returnvalue_2)))))

(fn `PrintFrequency`
  (params (frequency :type "Float (double-precision)"))
  (bind _returnvalue (* frequency 100.0))
  (if (>= _returnvalue 1.0)
    (`KismetSystemLibrary.PrintString` (`KismetStringLibrary.Conv_IntToString` (`KismetMathLibrary.Round` _returnvalue)))))

(fn `Spawn Notes`
  (params (freq_spawn_notes :type "Float (double-precision)"))
  (bind _returnvalue (* freq_spawn_notes 100.0))
  (bind _returnvalue_2 (`KismetMathLibrary.Round` _returnvalue))
  (bind _returnvalue_3 (* _returnvalue 1.0))
  (if (<= _returnvalue_2 5)
    (`FXSystemComponent.SetFloatParameter` (`self.note_particles`) "eighth_spawn" 0.5)
    (`FXSystemComponent.SetFloatParameter` (`self.note_particles`) "half_spawn" 0.5)
    (`FXSystemComponent.SetFloatParameter` (`self.note_particles`) "sixteenth_spawn" 0.5)
    (`self.VelocityNotes` _returnvalue)
    (`self.AccelerationNotes` _returnvalue)
    (elif (<= _returnvalue_2 10)
      (`FXSystemComponent.SetFloatParameter` (`self.note_particles`) "eighth_spawn" 2.0)
      (`FXSystemComponent.SetFloatParameter` (`self.note_particles`) "half_spawn" 2.0)
      (`FXSystemComponent.SetFloatParameter` (`self.note_particles`) "sixteenth_spawn" 2.0)
      (`self.VelocityNotes` _returnvalue)
      (`self.AccelerationNotes` _returnvalue)
      (elif (<= _returnvalue_2 20)
        (`FXSystemComponent.SetFloatParameter` (`self.note_particles`) "eighth_spawn" 5.0)
        (`FXSystemComponent.SetFloatParameter` (`self.note_particles`) "half_spawn" 5.0)
        (`FXSystemComponent.SetFloatParameter` (`self.note_particles`) "sixteenth_spawn" 5.0)
        (`self.VelocityNotes` _returnvalue)
        (`self.AccelerationNotes` _returnvalue)
        (elif (> _returnvalue_2 22)
          (`FXSystemComponent.SetFloatParameter` (`self.note_particles`) "eighth_spawn" _returnvalue_3)
          (`FXSystemComponent.SetFloatParameter` (`self.note_particles`) "half_spawn" _returnvalue_3)
          (`FXSystemComponent.SetFloatParameter` (`self.note_particles`) "sixteenth_spawn" _returnvalue_3)
          (`self.VelocityNotes` _returnvalue)
          (`self.AccelerationNotes` _returnvalue))))))

(fn `SpawnLeafFunction`
  (params (freq_spawn :type "Float (double-precision)"))
  (bind _returnvalue (/ (`KismetMathLibrary.Conv_IntToDouble` (`KismetMathLibrary.Round` (* freq_spawn 100.0))) 2.0))
  (`FXSystemComponent.SetFloatParameter` (`self.leaf_particles`) "leaf_spawn" _returnvalue)
  (`FXSystemComponent.SetFloatParameter` (`self.green_leaf_particles`) "green_leaf_spawn" _returnvalue))

(fn `SpawnWindFunction`
  (params (freq_spawn_wind :type "Float (double-precision)"))
  (if (>= (`KismetMathLibrary.Round` (* freq_spawn_wind 100.0)) 10)
    (`FXSystemComponent.SetFloatParameter` (`self.wind_line_particles`) "wind_point_spawn" 1.0)
    (`FXSystemComponent.SetFloatParameter` (`self.wind_line_particles`) "wind_line_spawn" 1.0)
    (else
      (`FXSystemComponent.SetFloatParameter` (`self.wind_line_particles`) "wind_point_spawn" 0.0)
      (`FXSystemComponent.SetFloatParameter` (`self.wind_line_particles`) "wind_line_spawn" 0.0))))

(fn `SpawnWindSwirls`
  (params (freq_spawn_swirl :type "Float (double-precision)"))
  (if (>= (`KismetMathLibrary.Round` (* freq_spawn_swirl 100.0)) 20)
    (`FXSystemComponent.SetFloatParameter` (`self.wind_swirls_particles`) "wind_swirl_point_spawn" 4.0)
    (`FXSystemComponent.SetFloatParameter` (`self.wind_swirls_particles`) "swirl_wind_spawn" 1.0)
    (else
      (`FXSystemComponent.SetFloatParameter` (`self.wind_swirls_particles`) "wind_swirl_point_spawn" 0.0)
      (`FXSystemComponent.SetFloatParameter` (`self.wind_swirls_particles`) "swirl_wind_spawn" 0.0))))

(fn `UserConstructionScript`)

(fn `VelocityNotes`
  (params (note_freq :type "Float (double-precision)"))
  (bind _returnvalue (`KismetMathLibrary.MakeVector` (`KismetMathLibrary.RandomFloatInRange` -20.0 20.0) 45.0))
  (bind _returnvalue_2 (`KismetMathLibrary.MakeVector` (`KismetMathLibrary.RandomFloatInRange` -50.0 50.0) 70.0 (`KismetMathLibrary.RandomFloatInRange` 0.0 note_freq)))
  (bind _returnvalue_3 (`KismetMathLibrary.MakeVector` (`KismetMathLibrary.RandomFloatInRange` -5.0 5.0) 30.0))
  (if (<= note_freq 10.0)
    (`FXSystemComponent.SetVectorParameter` (`self.note_particles`) "eighth_vel" _returnvalue_3)
    (`FXSystemComponent.SetVectorParameter` (`self.note_particles`) "half_vel" _returnvalue_3)
    (`FXSystemComponent.SetVectorParameter` (`self.note_particles`) "sixteenth_vel" _returnvalue_3)
    (elif (<= note_freq 20.0)
      (`FXSystemComponent.SetVectorParameter` (`self.note_particles`) "eighth_vel" _returnvalue)
      (`FXSystemComponent.SetVectorParameter` (`self.note_particles`) "half_vel" _returnvalue)
      (`FXSystemComponent.SetVectorParameter` (`self.note_particles`) "sixteenth_vel" _returnvalue)
      (elif (> note_freq 20.0)
        (`FXSystemComponent.SetVectorParameter` (`self.note_particles`) "eighth_vel" _returnvalue_2)
        (`FXSystemComponent.SetVectorParameter` (`self.note_particles`) "half_vel" _returnvalue_2)
        (`FXSystemComponent.SetVectorParameter` (`self.note_particles`) "sixteenth_vel" _returnvalue_2)))))