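; BP_ARScene is an AR scene Blueprint that reveals the content attached to it when its Enable function is called.
; Enable loops over attached actors and unhides each, then activates the particle system on Emitters or turns on mesh visibility, propagated to children, on StaticMeshActors.
; Audio activation and emitter visibility nodes are present but never run, and the construction script is empty.
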(fn `Enable`
  (for _array_element (`self.GetAttachedActors` true)
    (`self.SetActorHiddenInGame` _array_element false)
    (bind _asemitter (cast `Emitter` _array_element)
      (:`then`
        (`ActorComponent.Activate` (`Emitter.ParticleSystemComponent` _asemitter) false))
      (:`CastFailed`
        (bind _asstatic_mesh_actor (cast `StaticMeshActor` _array_element))
        (`SceneComponent.SetVisibility` (`StaticMeshActor.StaticMeshComponent` _asstatic_mesh_actor) true true)))))

(fn `UserConstructionScript`)