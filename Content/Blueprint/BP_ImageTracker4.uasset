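; Magic Leap image-tracking actor that anchors the AR scene to a detected image target.
; When the target is found, it enables the BP_ARScene actor in the level and shows its Cube.
; After a short delay, it moves the scene to the tracker's world location plus a fixed offset, leaving rotation untouched.
; Losing the target hides only the Cube.
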(event `self.MagicLeapImageTracker.OnImageTargetFound`
  (bind _returnvalue (`GameplayStatics.GetActorOfClass` "/Game/Blueprint/BP_ARScene.BP_ARScene_C"))
  (`/Game/Blueprint/BP_ARScene.Enable` _returnvalue)
  (`SceneComponent.SetHiddenInGame` (`self.Cube`) false true)
  (bind _returnvalue_2 (`GameplayStatics.GetActorOfClass` "/Game/Blueprint/BP_ARScene.BP_ARScene_C"))
  (`KismetSystemLibrary.Delay` 0.5)
  (`self.K2_SetActorLocation` _returnvalue_2 (+ (`SceneComponent.K2_GetComponentLocation` (`self.MagicLeapImageTracker`)) (400.0 0.0 -175.0)) false false))

(event `self.MagicLeapImageTracker.OnImageTargetLost`
  (`SceneComponent.SetHiddenInGame` (`self.Cube`) true true))

(fn `UserConstructionScript`)