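; XR pawn that re-bases its view once at startup from the player camera's initial pose.
; A one-shot on Tick sets the XRCamera world transform to the inverse of the camera manager's location and yaw, ignoring pitch and roll and using the component's scale.
; On Lumin (Magic Leap) this runs on the first tick, while other platforms use a flag to wait until the second.
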(event `self.ReceiveTick`
  (params (DeltaSeconds :type "Float (single-precision)"))
  (bind _returnvalue (`GameplayStatics.GetPlayerCameraManager` 0))
  (if (`KismetStringLibrary.EqualEqual_StrStr` (`GameplayStatics.GetPlatformName`) "Lumin")
    (`/Engine/EditorBlueprintResources/StandardMacros.DoOnce` false :!label _label
      (:`Completed`
        (`SceneComponent.K2_SetWorldTransform` (`self.XR_Camera`) (`KismetMathLibrary.InvertTransform` (`KismetMathLibrary.MakeTransform` (`PlayerCameraManager.GetCameraLocation` _returnvalue) (`KismetMathLibrary.MakeRotator` 0.0 0.0 (.yaw (`PlayerCameraManager.GetCameraRotation` _returnvalue))) (`SceneComponent.K2_GetComponentScale` (`self.XR_Camera`)))) false false)))
    (elif (`self.Is First Name`)
      (goto _label)
      (else
        (set `self.Is First Name` true)))))

(fn `UserConstructionScript`)